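; BP_BasketBallScore is a scoring trigger that awards points when a BP_BasketBall overlaps it.
; Each overlap adds a fixed amount to a running total, reset at BeginPlay, and writes it to the referenced ScoreBoard.
; It also plays a ding and spawns a scaled-down, time-dilated score effect at the ball's location.
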(event EventBeginPlay
  (Variables|Default|SetTotalScore 0.0))

(event Collision|EventActorBeginOverlap
  (params (OtherActor :type Actor%20Object%20Reference))
  (bind _returnvalue (Transformation|GetActorLocation OtherActor))
  (Utilities|Casting|CastToBP_BasketBall OtherActor)
  (bind _output_get (Variables|Default|SetTotalScore (+ (Variables|Default|GetTotalScore) 1e+02)))
  (Variables|/Game/Blueprints/BP_ScoreBoard.BP_ScoreBoard_C|SetScore (Variables|Default|GetScoreBoard) _output_get)
  (Audio|PlaySoundatLocation "/Game/ding.ding" _returnvalue "0, 0, 0" 1.0 1.0 0.0 0 0 0 0)
  (bind _returnvalue_2 (Niagara|SpawnSystematLocation "/Game/ScoreFX.ScoreFX" _returnvalue "0, 0, 0" "0.300000,0.300000,0.300000"))
  (Class|NiagaraComponent|SetCustomTimeDilation _returnvalue_2 3.0))

(event EventTick
  (params (DeltaSeconds :type Float%20%28single-precision%29)))

(fn ConstructionScript)