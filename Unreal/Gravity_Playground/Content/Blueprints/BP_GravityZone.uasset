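; BP_GravityZone is a zone actor that changes gravity for BP_CustomPhysics actors inside it.
; Begin and end overlap events maintain the ObjectsToAffect list, with a debug print on entry.
; Each tick it pushes each listed actor's static mesh with AntiGravity plus LocalGravity scaled by mass, so acceleration is mass-independent.
; An unconnected branch would gather already-overlapping actors but never runs.
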(event Collision|EventActorBeginOverlap
  (params (OtherActor :type Actor%20Object%20Reference))
  (bind _asbp_custom_physics (Utilities|Casting|CastToBP_CustomPhysics OtherActor))
  (Utilities|Array|AddUnique (Variables|Default|GetObjectsToAffect) _asbp_custom_physics)
  (Development|PrintString "Hello"))

(event Collision|EventActorEndOverlap
  (params (OtherActor :type Actor%20Object%20Reference))
  (bind _asbp_custom_physics (Utilities|Casting|CastToBP_CustomPhysics OtherActor))
  (Utilities|Array|RemoveItem (Variables|Default|GetObjectsToAffect) _asbp_custom_physics))

(event EventTick
  (params (DeltaSeconds :type Float%20%28single-precision%29))
  (for _array_element (Variables|Default|GetObjectsToAffect)
    (Physics|AddForce (Actor|GetComponentbyClass _array_element "/Script/Engine.StaticMeshComponent") (* (+ (Variables|Default|GetAntiGravity) (Variables|Default|GetLocalGravity)) (Physics|GetMass (Actor|GetComponentbyClass _array_element "/Script/Engine.StaticMeshComponent"))) "None" false)))

(event EventBeginPlay)

(fn ConstructionScript)